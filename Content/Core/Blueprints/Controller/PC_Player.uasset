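; Player controller that spawns and possesses its own BP_BaseCharacter and supports adding local players.
; On BeginPlay it uses its controller ID to pick a PlayerStart, falling back to the first one found if that index is invalid.
; MoveForward and MoveRight axes move the controlled pawn along the forward and right vectors of its control rotation.
; Pressing O creates another local player; an unconnected debug arrow for facing direction remains in the graph.
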(event EventBeginPlay
  (bind _outactors (Actor|GetAllActorsOfClass "/Script/Engine.PlayerStart"))
  (bind _output_get (Variables|Default|SetContorllerID (Class|GameplayStatics|GetPlayerControllerID self)))
  (bind _returnvalue (Game|SpawnActorfromClass "/Game/Core/Blueprints/Character/BP_BaseCharacter.BP_BaseCharacter_C" (Transformation|GetActorTransform (Utilities|Array|Get(acopy) _outactors (Math|Integer|SelectInt (Variables|Default|GetContorllerID) 0 (Utilities|Array|IsValidIndex _outactors _output_get)))) "Undefined" 0 0))
  (Pawn|Possess _returnvalue))

(event Input|AxisEvents|InputAxisMoveRight
  (params (AxisValue :type Float%20%28single-precision%29))
  (bind _returnvalue (Pawn|GetControlledPawn))
  (Pawn|Input|AddMovementInput _returnvalue (Math|Vector|GetRightVector (Pawn|GetControlRotation _returnvalue :!class /Script/Engine.Pawn)) AxisValue false))

(event Input|AxisEvents|InputAxisMoveForward
  (params (AxisValue :type Float%20%28single-precision%29))
  (bind _returnvalue (Pawn|GetControlledPawn))
  (Pawn|Input|AddMovementInput _returnvalue (Math|Vector|GetForwardVector (Pawn|GetControlRotation _returnvalue :!class /Script/Engine.Pawn)) AxisValue false))

(event Input|KeyboardEvents|F
  (params (Key :type Key%20Structure :default "None")))

(event Input|KeyboardEvents|O
  (params (Key :type Key%20Structure :default "None"))
  (:Pressed
    (Class|GameplayStatics|CreatePlayer -1)))

(fn ConstructionScript)