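; BP_GameCamera is a game camera actor that mirrors the transform of another actor in the level.
; On BeginPlay it stores the first actor tagged "Camera" as CameraParent, then copies that actor's transform immediately and again every Tick, without attachment.
; Unconnected leftover logic for attaching to an owning character and blending the player's view target to this camera never runs.
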(event EventBeginPlay
  (bind _outactors (Actor|GetAllActorswithTag "Camera"))
  (Variables|Default|SetCameraParent (Utilities|Array|Get(acopy) _outactors))
  (CallFunction|UpdateCameraTransform))

(event Collision|EventActorBeginOverlap
  (params (OtherActor :type Actor%20Object%20Reference)))

(event EventTick
  (params (DeltaSeconds :type Float%20%28single-precision%29))
  (CallFunction|UpdateCameraTransform))

(fn ConstructionScript)

(fn UpdateCameraTransform
  (Transformation|SetActorTransform (Transformation|GetActorTransform (Variables|Default|GetCameraParent))))